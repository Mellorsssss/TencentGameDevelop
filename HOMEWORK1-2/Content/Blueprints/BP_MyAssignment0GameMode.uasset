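; BP_MyAssignment0GameMode is a game mode that tracks the player's score and shows it on screen.
; On BeginPlay it creates BP_ScoreWidget and adds it to the viewport.
; The AddScore and SetScoreToZero events update PlayerScore and rewrite the widget's text with a Chinese "current score" label.
; RestartMyGame simply forwards to RestartTpsGame.
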(event Custom|AddScore
  (params (score :type Integer))
  (bind _output_get (Variables|Default|SetPlayerScore (+ score (Variables|Default|GetPlayerScore))))
  (Rendering|Components|TextRender|SetText (Variables|/Game/Blueprints/BP_ScoreWidget.BP_ScoreWidget_C|GetText (Variables|Default|GetGame_Score_Widget)) (Utilities|Text|ToText(String) (Utilities|String|Append "当前分数：" (Utilities|String|ToString(Integer) _output_get)))))

(event Custom|SetScoreToZero
  (bind _output_get (Variables|Default|SetPlayerScore 0))
  (Rendering|Components|TextRender|SetText (Variables|/Game/Blueprints/BP_ScoreWidget.BP_ScoreWidget_C|GetText (Variables|Default|GetGame_Score_Widget)) (Utilities|Text|ToText(String) (Utilities|String|Append "当前分数：" (Utilities|String|ToString(Integer) _output_get)))))

(event EventBeginPlay
  (bind _returnvalue (UserInterface|CreateWidget "/Game/Blueprints/BP_ScoreWidget.BP_ScoreWidget_C"))
  (bind _output_get (Variables|Default|SetGame_Score_Widget _returnvalue))
  (UserInterface|Viewport|AddtoViewport _output_get 0))

(event EventTick
  (params (DeltaSeconds :type Float%20%28single-precision%29)))

(fn ConstructionScript)

(fn RestartMyGame
  (Class|Assignment0GameMode|RestartTpsGame))