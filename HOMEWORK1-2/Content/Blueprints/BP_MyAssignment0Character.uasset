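; Player character Blueprint that adds a toggleable armed mode with gun firing.
; The Shooting input flips the Shoot flag and shows or hides Gunmesh to match.
; The Fire input calls Fire, which is not defined in these graphs, and plays a weapon sound at the character's location, only while armed.
; An unconnected, buggy-flagged draft that spawns BP_Wep onto the mesh's WeaponSocket never runs.
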(event EventBeginPlay)

(event Collision|EventActorBeginOverlap
  (params (OtherActor :type Actor%20Object%20Reference)))

(event EventTick
  (params (DeltaSeconds :type Float%20%28single-precision%29)))

(event Input|ActionEvents|InputActionFire
  (params (Key :type Key%20Structure :default "None"))
  (:Pressed
    (if (Variables|Default|GetShoot)
      (Class|Assignment0Character|Fire)
      (Audio|PlaySoundatLocation "/Game/Audio/GunShotAudio.FirstPersonTemplateWeaponFire02" (Transformation|GetActorLocation) "0, 0, 0" 1.0 1.0 0.0 0 0 0))))

(event Input|ActionEvents|InputActionShooting
  (params (Key :type Key%20Structure :default "None"))
  (:Pressed
    (if (Variables|Default|GetShoot)
      (Variables|Default|SetShoot false)
      (else
        (Variables|Default|SetShoot true)))
    (Rendering|SetVisibility (Variables|Default|GetGunmesh) (Variables|Default|GetShoot) false)))

(fn ConstructionScript)