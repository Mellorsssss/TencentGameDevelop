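; BP_Grenader is an AI-controlled grenadier character, built on a parent class, that runs the BT_Grenader behavior tree.
; On BeginPlay it starts the tree through its AI controller and seeds the TargetPosition blackboard key with a hardcoded vector.
; It also handles the Fire input press, calling BeginFire and firing CurrentWeapon while bullets remain.
; An EndFire call is present but unconnected.
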(event EventBeginPlay
  ;[1 1 1] 初始化行为树
  (AI|RunBehaviorTree (AI|GetAIController self) "/Game/AI/GrenadeAI/BT_Grenader.BT_Grenader")
  (AI|Components|Blackboard|SetValueasVector (AI|GetBlackboard self) (Utilities|Name|MakeLiteralName "TargetPosition") "0.000000,0.000000,236.001694"))

(event Input|ActionEvents|InputActionFire
  (params (Key :type Key%20Structure :default "None"))
  (:Pressed
    (Class|HOMEWORK3Character|BeginFire)
    (if (not (<= (Variables|Default|GetBulletNum) 0))
      (Class|TPSWeapon|Fire (Variables|Default|GetCurrentWeapon)))))

(fn ConstructionScript
  (|CallParentFunction))