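; BP_Sniper is a sniper character Blueprint, driven by AI, that extends a parent with weapon and ammo logic.
; On the authority, BeginPlay waits briefly, runs BT_Sniper through its AI controller and seeds the TargetPosition blackboard key with a fixed vector.
; A Fire input press also calls BeginFire and fires the current weapon while bullets remain.
; EndFire is left unconnected, and a custom event prints a debug greeting.
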(event Custom|自定义事件_0
  (Development|PrintString "Hello"))

(event EventBeginPlay
  ;[1 1 1] 初始化行为树
  (Networking|SwitchHasAuthority
    (:Authority
      (Utilities|FlowControl|Delay 1.0)
      (CallFunction|自定义事件0)
      (AI|RunBehaviorTree (AI|GetAIController self) "/Game/AI/SniperAI/BT_Sniper.BT_Sniper")
      (AI|Components|Blackboard|SetValueasVector (AI|GetBlackboard self) (Utilities|Name|MakeLiteralName "TargetPosition") "0.000000,0.000000,236.001694"))))

(event Input|ActionEvents|InputActionFire
  (params (Key :type Key%20Structure :default "None"))
  (:Pressed
    (Class|HOMEWORK3Character|BeginFire)
    (if (not (<= (Variables|Default|GetBulletNum) 0))
      (Class|TPSWeapon|Fire (Variables|Default|GetCurrentWeapon)))))

(fn ConstructionScript
  (|CallParentFunction))