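; Game state for a third-person shooter that ends the game and updates a saved scoreboard when the player runs out of bullets.
; Tick watches the character's bullet count and, once, fetches the player name from BP_PlayState and calls SaveGameData.
; That rebuilds the "ScoreBoard" save, inserting the current score before the first equal or lower record, or creating the slot if loading fails.
; It then shows the game-over widget with the scores, pauses and enables the cursor.
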(event EventTick
  (params (DeltaSeconds :type Float%20%28single-precision%29))
  (bind _asbp_tpscharacter (Utilities|Casting|CastToBP_TPSCharacter (Pawn|GetControlledPawn (Game|GetPlayerController 0))))
  (if (<= (Variables|/Script/HOMEWORK3.HOMEWORK3Character|GetBulletNum _asbp_tpscharacter) 0)
    (Utilities|FlowControl|DoOnce false
      (:Completed
        (bind _return (CallFunction|GetPlayerCurrentName))
        (Variables|Default|SetName _return)
        (CallFunction|SaveGameData)))))

(fn ConstructionScript)

(fn SaveGameData
  (bind _returnvalue (Game|GetPlayerController 0))
  (bind _tempdata (Variables|Default|GetTempData))
  (bind _playerstate (Variables|/Script/Engine.Controller|GetPlayerState _returnvalue))
  (bind _score (Variables|/Script/Engine.PlayerState|GetScore _playerstate))
  (bind _returnvalue_2 (SaveGame|LoadGamefromSlot "ScoreBoard"))
  (bind _asscore_sava_data (Utilities|Casting|CastToScoreSavaData _returnvalue_2)
    (:then
      (for _array_element (Variables|/Game/UI/DataStruct/ScoreSavaData.ScoreSavaData_C|GetPlayerScores _asscore_sava_data)
        (Utilities|FlowControl|Sequence
          (:then_0
            (if (<= (.Score (Utilities|Struct|BreakScoreRecord _array_element)) _score)
              (Utilities|FlowControl|DoOnce false
                (:Completed
                  (Utilities|Array|Add _tempdata (Utilities|Struct|MakeScoreRecord (Variables|Default|GetName) _score))))))
          (:then_1
            (Utilities|Array|Add _tempdata _array_element))))
      (bind _returnvalue_3 (SaveGame|CreateSaveGameObject "/Game/UI/DataStruct/ScoreSavaData.ScoreSavaData_C" :!label _label))
      (bind _asscore_sava_data_2 (Utilities|Casting|CastToScoreSavaData _returnvalue_3))
      (Variables|/Game/UI/DataStruct/ScoreSavaData.ScoreSavaData_C|SetPlayerScores _asscore_sava_data_2 (Variables|Default|GetTempData))
      (SaveGame|SaveGametoSlot _returnvalue_3 "ScoreBoard")
      (bind _returnvalue_4 (UserInterface|CreateWidget "/Game/GameJamKit/Blueprints/UMG/UMG_GameJam_GameOver_Widget.UMG_GameJam_GameOver_Widget_C" 0 (Variables|Default|GetTempData)))
      (bind _output_get (Variables|Default|SetGameOverWidget _returnvalue_4))
      (UserInterface|Viewport|AddtoViewport _output_get 0)
      (CallFunction|GameOver "少侠，你没有子弹了！"))
    (:CastFailed
      (Utilities|FlowControl|Sequence ; 如果打开插槽失败，那么直接创建该插槽
        (:then_0
          (Utilities|FlowControl|DoOnce false
            (:Completed
              (Utilities|Array|Add _tempdata (Utilities|Struct|MakeScoreRecord (Variables|Default|GetName) _score)))))
        (:then_1
          (goto _label))))))

(fn GetPlayerCurrentName
  (bind _asbp_play_state (Utilities|Casting|CastToBP_PlayState (Variables|/Script/Engine.Controller|GetPlayerState (Game|GetPlayerController 0))))
  (Development|PrintString (Utilities|String|ToString(Text) (Utilities|Text|ToText(String) (Class|TPSPlayerState|GetName _asbp_play_state))))
  (return (Utilities|Text|ToText(String) (Class|TPSPlayerState|GetName _asbp_play_state))))

(fn GameOver
  (params (LabelText :type Text))
  (bind _gameoverwidget (Variables|Default|GetGameOverWidget))
  (bind _returnvalue (Widget|GetOwningPlayer _gameoverwidget))
  ;[1 1 1] Game Over
  (Rendering|Components|TextRender|SetText (Variables|/Game/GameJamKit/Blueprints/UMG/UMG_GameJam_GameOver_Widget.UMG_GameJam_GameOver_Widget_C|GetLabelText _gameoverwidget) LabelText)
  (Game|SetGamePaused true)
  (Variables|/Script/Engine.PlayerController|SetbShowMouseCursor _returnvalue true)
  (Input|SetInputModeGameandUI _returnvalue _gameoverwidget "DoNotLock" false))