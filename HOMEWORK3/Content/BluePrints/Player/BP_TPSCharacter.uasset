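; Player character Blueprint for a third-person shooter, handling fire input and touch-drag camera look.
; Fire press calls BeginFire, sets the PlayerController InfoWidget's bullet bar from the ammo ratio, then fires CurrentWeapon; release calls EndFire.
; Touch movement deltas, scaled by turn rate and frame time, drive controller pitch and yaw.
; HUD creation nodes are disconnected, and a note marks the ammo UI logic for migration to C++.
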(event Input|ActionEvents|InputActionFire
  (params (Key :type Key%20Structure :default "None"))
  ;[1 1 1] 设置剩余子弹UI
  (:Pressed
    (Class|HOMEWORK3Character|BeginFire)
    (bind _asbp_player_controller (Utilities|Casting|CastToBP_PlayerController (Game|GetPlayerController 0)))
    (Progress|SetPercent (Variables|/Game/UI/BP_InfoWidget.BP_InfoWidget_C|GetBulletBar (Variables|/Game/BluePrints/Player/BP_PlayerController.BP_PlayerController_C|GetInfoWidget _asbp_player_controller)) (* (Variables|Default|GetBulletNum) (/ 1.0 (Math|Conversions|ToFloat(Integer) (Variables|Default|GetTotalBulletNum)))))
    ;[1 1 1] 自动开火
    (Class|TPSWeapon|Fire (Variables|Default|GetCurrentWeapon)))
  (:Released
    (Class|HOMEWORK3Character|EndFire)))

(event Input|TouchEvents|InputTouch
  (params (Location :type Vector) (FingerIndex :type ETouchIndex%20Enum))
  (bind _returnvalue (Utilities|Time|GetWorldDeltaSeconds))
  ;[1 1 1] 实现触屏移动视角
  (:Pressed
    (Variables|Default|SetTouchLocation Location))
  (:Moved
    (Pawn|Input|AddControllerPitchInput (* (.Y (Math|Vector|BreakVector (- (Variables|Default|GetTouchLocation) Location))) (Variables|Default|GetTouchTurnRate) _returnvalue))
    (Pawn|Input|AddControllerYawInput (* (.X (Math|Vector|BreakVector (- (Variables|Default|GetTouchLocation) Location))) (Variables|Default|GetTouchTurnRate) _returnvalue))
    (Variables|Default|SetTouchLocation Location)))

(fn ConstructionScript)