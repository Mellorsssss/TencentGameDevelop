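; BP_TPSCharacter is a third-person shooter character that spawns with a weapon and fires it with limited ammo.
; On BeginPlay it spawns BP_BasicWeapon with collision ignored and attaches it to the mesh's WeaponSocket.
; Fire input, while bullets remain, decrements the count, updates the player controller's InfoWidget bullet bar and calls the weapon's Fire.
; Crosshair and info widget creation is left here as unconnected nodes.
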(event EventBeginPlay
  (Utilities|FlowControl|Sequence
    (:then_1
      (bind _returnvalue (Game|SpawnActorfromClass "/Game/BluePrints/BP_BasicWeapon.BP_BasicWeapon_C" (Math|Transform|MakeTransform "0, 0, 0") "AlwaysSpawn" self 0)) ; 生成武器，注意需要忽略碰撞
      (bind _output_get (Variables|Default|SetCurrentWeapon _returnvalue))
      (Transformation|AttachComponentToComponent _output_get (Variables|Character|GetMesh) "WeaponSocket" "KeepRelative" "KeepRelative" "KeepRelative" true))))

(event Collision|EventActorBeginOverlap
  (params (OtherActor :type Actor%20Object%20Reference)))

(event EventTick
  (params (DeltaSeconds :type Float%20%28single-precision%29)))

(event Input|ActionEvents|InputActionFire
  (params (Key :type Key%20Structure :default "None"))
  (:Pressed
    (if (> (Variables|Default|GetBulletNum) 0)
      (Variables|Default|SetBulletNum (- (Variables|Default|GetBulletNum) 1))
      (bind _asbp_player_controller (Utilities|Casting|CastToBP_PlayerController (Game|GetPlayerController 0)))
      (Progress|SetPercent (Variables|/Game/UI/BP_InfoWidget.BP_InfoWidget_C|GetBulletBar (Variables|/Game/BluePrints/BP_PlayerController.BP_PlayerController_C|GetInfoWidget _asbp_player_controller)) (* (- (Variables|Default|GetBulletNum) 1) 0.05))
      (Class|TPSWeapon|Fire (Variables|Default|GetCurrentWeapon)))))

(fn ConstructionScript)