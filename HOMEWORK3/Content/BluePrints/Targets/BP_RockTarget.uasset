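; BP_RockTarget is a moving shooting target that awards score when hit.
; Point damage casts from the causing BP_BasicWeapon through its owning BP_TPSCharacter to TPSPlayerState and adds the damage as score.
; Tick offsets the actor from its skeletal mesh location by Direction times Speed per frame, without delta-time scaling.
; A Delay in Tick feeds a FlipFlop that reverses Direction along X about every two seconds.
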(event EventBeginPlay)

(event Collision|EventActorBeginOverlap
  (params (OtherActor :type Actor%20Object%20Reference)))

(event Game|Damage|EventPointDamage
  (params (Damage :type Float%20%28single-precision%29) (DamageType :type Damage%20Type%20Object%20Reference) (HitLocation :type Vector :default "0, 0, 0") (HitNormal :type Vector :default "0, 0, 0") (HitComponent :type Primitive%20Component%20Object%20Reference) (BoneName :type Name :default "None") (ShotFromDirection :type Vector :default "0, 0, 0") (InstigatedBy :type Controller%20Object%20Reference) (DamageCauser :type Actor%20Object%20Reference) (HitInfo :type Hit%20Result%20Structure%20%28by%20ref%29))
  (Utilities|FlowControl|Sequence
    (:then_1
      (bind _asbp_basic_weapon (Utilities|Casting|CastToBP_BasicWeapon DamageCauser))
      (bind _asbp_tpscharacter (Utilities|Casting|CastToBP_TPSCharacter (Components|GetOwner _asbp_basic_weapon)))
      (bind _astpsplayer_state (Utilities|Casting|CastToTPSPlayerState (Variables|/Script/Engine.Pawn|GetPlayerState _asbp_tpscharacter)))
      (Class|TPSPlayerState|AddScore _astpsplayer_state Damage))))

(event EventTick
  (params (DeltaSeconds :type Float%20%28single-precision%29))
  (Transformation|SetActorLocation (+ (Transformation|GetWorldLocation (Variables|Default|GetSkeletalMesh)) (* (Variables|Default|GetDirection) (Variables|Default|GetSpeed))) false false)
  (Utilities|FlowControl|Delay 2.0)
  (Utilities|FlowControl|FlipFlop
    (:A
      (Variables|Default|SetDirection "-1.000000,0.000000,0.000000"))
    (:B
      (Variables|Default|SetDirection "1.000000, 0, 0"))))

(fn ConstructionScript)

(fn Move)