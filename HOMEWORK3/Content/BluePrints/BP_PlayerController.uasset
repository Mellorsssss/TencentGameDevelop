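; Player controller that creates the local player's HUD and syncs it with the player state.
; On BeginPlay, local controllers add an info widget and a crosshair widget to the viewport.
; Every Tick it writes the PlayerState score into the info widget, then casts to BP_PlayState and sets its name from the widget's edited name text, polling rather than using events.
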(event EventBeginPlay
  (CallFunction|SetupGameUI))

(event EventTick
  (params (DeltaSeconds :type Float%20%28single-precision%29))
  (Rendering|Components|TextRender|SetText (Variables|/Game/UI/BP_InfoWidget.BP_InfoWidget_C|GetScoreText (Variables|Default|GetInfoWidget)) (Utilities|Text|ToText(String) (Utilities|String|ToString(Float) (Variables|/Script/Engine.PlayerState|GetScore (Variables|Default|GetPlayerState)))))
  (bind _asbp_play_state (Utilities|Casting|CastToBP_PlayState (Variables|Default|GetPlayerState)))
  (Class|TPSPlayerState|SetName _asbp_play_state (Utilities|String|ToString(Text) (Class|EditableText|GetText (Variables|/Game/UI/BP_InfoWidget.BP_InfoWidget_C|GetEditedName (Variables|Default|GetInfoWidget))))))

(fn ConstructionScript)

(fn SetupGameUI
  (if (Pawn|IsLocalPlayerController)
    (bind _returnvalue (UserInterface|CreateWidget "/Game/UI/BP_InfoWidget.BP_InfoWidget_C" self))
    (Variables|Default|SetInfoWidget _returnvalue)
    (UserInterface|Viewport|AddtoViewport (Variables|Default|GetInfoWidget) 0)
    (bind _returnvalue_2 (UserInterface|CreateWidget "/Game/UI/BP_CrossHair.BP_CrossHair_C" self))
    (Variables|Default|SetCrossHair _returnvalue_2)
    (UserInterface|Viewport|AddtoViewport (Variables|Default|GetCrossHair) 0)))