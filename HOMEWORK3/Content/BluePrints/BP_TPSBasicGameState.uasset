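; TPS game state that handles game over and the saved high-score board once the player character runs out of bullets.
; Tick polls the bullet count and, on every frame it is zero or below, shows the HUD score message and reruns the save flow.
; A DoOnce inserts the player's record before the first saved score it matches or beats, or alone without save data.
; TempData then overwrites the ScoreBoard slot and feeds a new BP_ScoreBoard widget.
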(event EventBeginPlay)

(event EventTick
  (params (DeltaSeconds :type Float%20%28single-precision%29))
  (bind _returnvalue (Game|GetPlayerController 0))
  (bind _returnvalue_2 (Game|GetPlayerController 0))
  (bind _tempdata (Variables|Default|GetTempData))
  (bind _playerstate (Variables|/Script/Engine.Controller|GetPlayerState _returnvalue_2))
  (bind _score (Variables|/Script/Engine.PlayerState|GetScore _playerstate))
  (bind _asbp_tpscharacter (Utilities|Casting|CastToBP_TPSCharacter (Pawn|GetControlledPawn _returnvalue)))
  (if (<= (Variables|/Game/BluePrints/BP_TPSCharacter.BP_TPSCharacter_C|GetBulletNum _asbp_tpscharacter) 0)
    (Class|BPGameJamKitHUDInterface|ShowGameOver(Message) (HUD|GetHUD _returnvalue) (Utilities|Text|ToText(String) (Utilities|String|Append "你的分数：" (Utilities|String|ToString(Float) (Variables|/Script/Engine.PlayerState|GetScore (Variables|/Script/Engine.Controller|GetPlayerState _returnvalue))))))
    (bind _returnvalue_3 (SaveGame|LoadGamefromSlot "ScoreBoard"))
    (bind _asscore_sava_data (Utilities|Casting|CastToScoreSavaData _returnvalue_3)
      (:then
        (for _array_element (Variables|/Game/UI/DataStruct/ScoreSavaData.ScoreSavaData_C|GetPlayerScores _asscore_sava_data)
          (Utilities|FlowControl|Sequence
            (:then_0
              (if (<= (.Score (Utilities|Struct|BreakScoreRecord _array_element)) _score)
                (Utilities|FlowControl|DoOnce false
                  (:Completed
                    (Utilities|Array|Add _tempdata (Utilities|Struct|MakeScoreRecord (Class|EditableText|GetText (Variables|/Game/UI/BP_InfoWidget.BP_InfoWidget_C|GetEditedName (Variables|/Game/BluePrints/BP_TPSCharacter.BP_TPSCharacter_C|GetInfoWidget _asbp_tpscharacter))) _score))))))
            (:then_1
              (Utilities|Array|Add _tempdata _array_element))))
        (bind _returnvalue_4 (SaveGame|CreateSaveGameObject "/Game/UI/DataStruct/ScoreSavaData.ScoreSavaData_C" :!label _label))
        (bind _asscore_sava_data_2 (Utilities|Casting|CastToScoreSavaData _returnvalue_4))
        (Variables|/Game/UI/DataStruct/ScoreSavaData.ScoreSavaData_C|SetPlayerScores _asscore_sava_data_2 (Variables|Default|GetTempData))
        (SaveGame|SaveGametoSlot _returnvalue_4 "ScoreBoard")
        (bind _returnvalue_5 (UserInterface|CreateWidget "/Game/UI/BP_ScoreBoard.BP_ScoreBoard_C" 0 (Variables|Default|GetTempData)))
        (UserInterface|Viewport|AddtoViewport _returnvalue_5 0))
      (:CastFailed
        (Utilities|FlowControl|Sequence ; 如果打开插槽失败，那么直接创建该插槽
          (:then_0
            (Utilities|FlowControl|DoOnce false
              (:Completed
                (Utilities|Array|Add _tempdata (Utilities|Struct|MakeScoreRecord (Class|EditableText|GetText (Variables|/Game/UI/BP_InfoWidget.BP_InfoWidget_C|GetEditedName (Variables|/Game/BluePrints/BP_TPSCharacter.BP_TPSCharacter_C|GetInfoWidget _asbp_tpscharacter))) _score)))))
          (:then_1
            (goto _label)))))))

(fn ConstructionScript)